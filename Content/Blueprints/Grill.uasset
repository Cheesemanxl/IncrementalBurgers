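; Grill actor for a Paper2D burger cooking game that displays the cooking state and the burger being made.
; Each Tick it polls BC_GameInstance, switching the grill flipbook between cooking and off animations based on IsCooking.
; When not cooking, it also sets the burger sprite's color according to IsDone.
; A switch on the BurgerStates enum picks the burger sprite for each combination of C, L, T and O toppings.
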(event `self.ReceiveTick`
  (params (DeltaSeconds :type "Float (single-precision)"))
  (`self.Grill Animation Handler`)
  (`self.Burger Animation Handler`)
  (bind _asbc_game_instance (cast `/Game/Blueprints/BC_GameInstance` (`GameplayStatics.GetGameInstance`)))
  (if (`/Game/Blueprints/BC_GameInstance.isDone` _asbc_game_instance)
    _))

(fn `Burger Animation Handler`
  (bind _burger_sprite (`self.Burger Sprite`))
  (bind _asbc_game_instance (cast `/Game/Blueprints/BC_GameInstance` (`GameplayStatics.GetGameInstance`)))
  (switch `/Game/Blueprints/Burger_States` (`/Game/Blueprints/BC_GameInstance.Burger States` _asbc_game_instance)
    (:`NewEnumerator0`
      (`PaperSpriteComponent.SetSprite` _burger_sprite "/Game/Sprites/Burger_Sprites/BASE.BASE"))
    (:`NewEnumerator1`
      (`PaperSpriteComponent.SetSprite` _burger_sprite "/Game/Sprites/Burger_Sprites/C.C"))
    (:`NewEnumerator2`
      (`PaperSpriteComponent.SetSprite` _burger_sprite "/Game/Sprites/Burger_Sprites/L.L"))
    (:`NewEnumerator3`
      (`PaperSpriteComponent.SetSprite` _burger_sprite "/Game/Sprites/Burger_Sprites/T.T"))
    (:`NewEnumerator4`
      (`PaperSpriteComponent.SetSprite` _burger_sprite "/Game/Sprites/Burger_Sprites/O.O"))
    (:`NewEnumerator5`
      (`PaperSpriteComponent.SetSprite` _burger_sprite "/Game/Sprites/Burger_Sprites/CL.CL"))
    (:`NewEnumerator6`
      (`PaperSpriteComponent.SetSprite` _burger_sprite "/Game/Sprites/Burger_Sprites/CO.CO"))
    (:`NewEnumerator7`
      (`PaperSpriteComponent.SetSprite` _burger_sprite "/Game/Sprites/Burger_Sprites/CT.CT"))
    (:`NewEnumerator8`
      (`PaperSpriteComponent.SetSprite` _burger_sprite "/Game/Sprites/Burger_Sprites/LO.LO"))
    (:`NewEnumerator9`
      (`PaperSpriteComponent.SetSprite` _burger_sprite "/Game/Sprites/Burger_Sprites/LT.LT"))
    (:`NewEnumerator10`
      (`PaperSpriteComponent.SetSprite` _burger_sprite "/Game/Sprites/Burger_Sprites/TO.TO"))
    (:`NewEnumerator11`
      (`PaperSpriteComponent.SetSprite` _burger_sprite "/Game/Sprites/Burger_Sprites/CLO.CLO"))
    (:`NewEnumerator12`
      (`PaperSpriteComponent.SetSprite` _burger_sprite "/Game/Sprites/Burger_Sprites/CLT.CLT"))
    (:`NewEnumerator13`
      (`PaperSpriteComponent.SetSprite` _burger_sprite "/Game/Sprites/Burger_Sprites/CTO.CTO"))
    (:`NewEnumerator14`
      (`PaperSpriteComponent.SetSprite` _burger_sprite "/Game/Sprites/Burger_Sprites/LTO.LTO"))
    (:`NewEnumerator15`
      (`PaperSpriteComponent.SetSprite` _burger_sprite "/Game/Sprites/Burger_Sprites/CLTO.CLTO"))))

(fn `Grill Animation Handler`
  (bind _grill_flipbook (`self.Grill Flipbook`))
  (bind _burger_sprite (`self.Burger Sprite`))
  (bind _asbc_game_instance (cast `/Game/Blueprints/BC_GameInstance` (`GameplayStatics.GetGameInstance`)))
  (if (`/Game/Blueprints/BC_GameInstance.isCooking` _asbc_game_instance)
    (`PaperFlipbookComponent.SetFlipbook` _grill_flipbook "/Game/Sprites/Cook_Anim.Cook_Anim")
    (else
      (`PaperFlipbookComponent.SetFlipbook` _grill_flipbook "/Game/Sprites/Off_Anim.Off_Anim")
      (if (`/Game/Blueprints/BC_GameInstance.isDone` _asbc_game_instance)
        (`PaperSpriteComponent.SetSpriteColor` _burger_sprite (make `LinearColor` 1.0 1.0 1.0 1.0))
        (else
          (`PaperSpriteComponent.SetSpriteColor` _burger_sprite (make `LinearColor` 1.0 1.0 1.0)))))))

(fn `UserConstructionScript`)
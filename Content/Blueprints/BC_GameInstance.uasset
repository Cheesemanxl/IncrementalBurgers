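; Game Instance for a burger business sim, holding the economy: ingredient purchases, cooking, stock, sales and upgrades.
; Topping unlocks select a BurgerStates enum, which sets the ingredients cooking requires, though a hardwired branch makes the bun check always pass.
; Incremental cooking yields burgers for collection, and a looping timer rolls each customer against appeal to sell stock.
; Price drives appeal and public demand, while topping and tiered advertising purchases raise base appeal.
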(fn `Begin Sell Loop`
  (`KismetSystemLibrary.K2_SetTimer` null "Sell Logic" 3.0 true))

(fn `Burger Price Appeal Logic`
  (bind _burger_price (`self.Burger Price`))
  (bind _base_appeal (`self.Base Appeal`))
  (if (<= _burger_price 1.0)
    (bind _output_get (set `self.Appeal Mod` (- 2.0 _burger_price)))
    (set `self.Current Appeal` (* _base_appeal _output_get))
    (else
      (bind _output_get_2 (set `self.Appeal Mod` (/ _base_appeal _burger_price)))
      (set `self.Current Appeal` _output_get_2))))

(fn `Burger State Logic`
  (bind _lettuceunlocked (`self.LettuceUnlocked`))
  (bind _tomatounlocked (`self.TomatoUnlocked`))
  (bind _onionunlocked (`self.OnionUnlocked`))
  ;[1 1 1] Chooses state of the Burger States ENUM based on which of the upgrades' unlocked variables are TRUE / assits with animation
  (if (`self.CheeseUnlocked`)
    (set `self.Burger States` "NewEnumerator1")
    (if _lettuceunlocked
      (set `self.Burger States` "NewEnumerator5")
      (if _tomatounlocked
        (set `self.Burger States` "NewEnumerator12")
        (if _onionunlocked
          (set `self.Burger States` "NewEnumerator15"))
        (elif _onionunlocked
          (set `self.Burger States` "NewEnumerator11")))
      (elif _tomatounlocked
        (set `self.Burger States` "NewEnumerator7")
        (if _onionunlocked
          (set `self.Burger States` "NewEnumerator13"))
        (elif _onionunlocked
          (set `self.Burger States` "NewEnumerator6"))))
    (elif _lettuceunlocked
      (set `self.Burger States` "NewEnumerator2")
      (if _tomatounlocked
        (set `self.Burger States` "NewEnumerator9")
        (if _onionunlocked
          (set `self.Burger States` "NewEnumerator14"))
        (elif _onionunlocked
          (set `self.Burger States` "NewEnumerator8")))
      (elif _tomatounlocked
        (set `self.Burger States` "NewEnumerator3")
        (if _onionunlocked
          (set `self.Burger States` "NewEnumerator10"))
        (elif _onionunlocked
          (set `self.Burger States` "NewEnumerator4")
          (else
            (set `self.Burger States` "NewEnumerator0")))))))

(fn `Buy Beef`
  (bind _cash (`self.Cash`))
  (if (>= (`KismetMathLibrary.Conv_IntToDouble` (`KismetMathLibrary.FTrunc` _cash)) 1.0)
    (`/Engine/EditorBlueprintResources/StandardMacros.DecrementFloat` _cash
      (:`  `
        (set `self.Beef` (+ (`self.Beef`) 2.0))))))

(fn `Buy Buns`
  (bind _cash (`self.Cash`))
  (if (>= (`KismetMathLibrary.Conv_IntToDouble` (`KismetMathLibrary.FTrunc` _cash)) 1.0)
    (`/Engine/EditorBlueprintResources/StandardMacros.DecrementFloat` _cash
      (:`  `
        (set `self.Buns` (+ (`self.Buns`) 10))))))

(fn `Buy Cheese`
  (bind _cash (`self.Cash`))
  (if (>= (`KismetMathLibrary.Conv_IntToDouble` (`KismetMathLibrary.FTrunc` _cash)) 1.0)
    (`/Engine/EditorBlueprintResources/StandardMacros.DecrementFloat` _cash
      (:`  `
        (set `self.Cheese` (+ (`self.Cheese`) 5))))))

(fn `Buy Lettuce`
  (bind _cash (`self.Cash`))
  (if (>= (`KismetMathLibrary.Conv_IntToDouble` (`KismetMathLibrary.FTrunc` _cash)) 1.0)
    (`/Engine/EditorBlueprintResources/StandardMacros.DecrementFloat` _cash
      (:`  `
        (set `self.Lettuce` (+ (`self.Lettuce`) 20))))))

(fn `Buy Onion`
  (bind _cash (`self.Cash`))
  (if (>= _cash 1.0)
    (`/Engine/EditorBlueprintResources/StandardMacros.DecrementFloat` _cash
      (:`  `
        (set `self.Onion` (+ (`self.Onion`) 10))))))

(fn `Buy Tomato`
  (bind _cash (`self.Cash`))
  (if (>= (`KismetMathLibrary.Conv_IntToDouble` (`KismetMathLibrary.FTrunc` _cash)) 1.0)
    (`/Engine/EditorBlueprintResources/StandardMacros.DecrementFloat` _cash
      (:`  `
        (set `self.Tomato` (+ (`self.Tomato`) 20))))))

(fn `Check Avaliable Ingredients`
  (if (>= (`self.Buns`) 1)
    (set `self.Ing Avail Buns` true)
    (else
      (set `self.Ing Avail Buns` false)))
  (if (>= (`self.Beef`) 0.5)
    (set `self.Ing Avail Beef` true)
    (else
      (set `self.Ing Avail Beef` false)))
  (if true
    (set `self.Ing Avail Buns` true)
    (else
      (set `self.Ing Avail Buns` false)))
  (if (>= (`self.Cheese`) 1)
    (set `self.Ing Avail Cheese` true)
    (else
      (set `self.Ing Avail Cheese` false)))
  (if (>= (`self.Lettuce`) 2)
    (set `self.Ing Avail Lettuce` true)
    (else
      (set `self.Ing Avail Lettuce` false)))
  (if (>= (`self.Tomato`) 2)
    (set `self.Ing Avail Tomato` true)
    (else
      (set `self.Ing Avail Tomato` false)))
  (if (>= (`self.Onion`) 1)
    (set `self.Ing Avail Onion` true)
    (else
      (set `self.Ing Avail Onion` false)))
  (switch `/Game/Blueprints/Burger_States` (`self.Burger States`)
    (:`NewEnumerator0`
      (if (and (`self.Ing Avail Beef`) (`self.Ing Avail Buns`))
        (set `self.Ingredients Avaliable` true)
        (else
          (set `self.Ingredients Avaliable` false))))
    (:`NewEnumerator1`
      (if (and (`self.Ing Avail Buns`) (`self.Ing Avail Cheese`) (`self.Ing Avail Beef`))
        (set `self.Ingredients Avaliable` true)
        (else
          (set `self.Ingredients Avaliable` false))))
    (:`NewEnumerator2`
      (if (and (`self.Ing Avail Buns`) (`self.Ing Avail Lettuce`) (`self.Ing Avail Beef`))
        (set `self.Ingredients Avaliable` true)
        (else
          (set `self.Ingredients Avaliable` false))))
    (:`NewEnumerator3`
      (if (and (`self.Ing Avail Buns`) (`self.Ing Avail Tomato`) (`self.Ing Avail Beef`))
        (set `self.Ingredients Avaliable` true)
        (else
          (set `self.Ingredients Avaliable` false))))
    (:`NewEnumerator4`
      (if (and (`self.Ing Avail Buns`) (`self.Ing Avail Onion`) (`self.Ing Avail Beef`))
        (set `self.Ingredients Avaliable` true)
        (else
          (set `self.Ingredients Avaliable` false))))
    (:`NewEnumerator5`
      (if (and (`self.Ing Avail Buns`) (`self.Ing Avail Cheese`) (`self.Ing Avail Lettuce`) (`self.Ing Avail Beef`))
        (set `self.Ingredients Avaliable` true)
        (else
          (set `self.Ingredients Avaliable` false))))
    (:`NewEnumerator6`
      (if (and (`self.Ing Avail Buns`) (`self.Ing Avail Cheese`) (`self.Ing Avail Onion`) (`self.Ing Avail Beef`))
        (set `self.Ingredients Avaliable` true)
        (else
          (set `self.Ingredients Avaliable` false))))
    (:`NewEnumerator7`
      (if (and (`self.Ing Avail Buns`) (`self.Ing Avail Cheese`) (`self.Ing Avail Tomato`) (`self.Ing Avail Beef`))
        (set `self.Ingredients Avaliable` true)
        (else
          (set `self.Ingredients Avaliable` false))))
    (:`NewEnumerator8`
      (if (and (`self.Ing Avail Buns`) (`self.Ing Avail Lettuce`) (`self.Ing Avail Onion`) (`self.Ing Avail Beef`))
        (set `self.Ingredients Avaliable` true)
        (else
          (set `self.Ingredients Avaliable` false))))
    (:`NewEnumerator9`
      (if (and (`self.Ing Avail Buns`) (`self.Ing Avail Lettuce`) (`self.Ing Avail Tomato`) (`self.Ing Avail Beef`))
        (set `self.Ingredients Avaliable` true)
        (else
          (set `self.Ingredients Avaliable` false))))
    (:`NewEnumerator10`
      (if (and (`self.Ing Avail Buns`) (`self.Ing Avail Tomato`) (`self.Ing Avail Onion`) (`self.Ing Avail Beef`))
        (set `self.Ingredients Avaliable` true)
        (else
          (set `self.Ingredients Avaliable` false))))
    (:`NewEnumerator11`
      (if (and (`self.Ing Avail Buns`) (`self.Ing Avail Cheese`) (`self.Ing Avail Lettuce`) (`self.Ing Avail Onion`) (`self.Ing Avail Beef`))
        (set `self.Ingredients Avaliable` true)
        (else
          (set `self.Ingredients Avaliable` false))))
    (:`NewEnumerator12`
      (if (and (`self.Ing Avail Buns`) (`self.Ing Avail Cheese`) (`self.Ing Avail Lettuce`) (`self.Ing Avail Tomato`) (`self.Ing Avail Beef`))
        (set `self.Ingredients Avaliable` true)
        (else
          (set `self.Ingredients Avaliable` false))))
    (:`NewEnumerator13`
      (if (and (`self.Ing Avail Buns`) (`self.Ing Avail Cheese`) (`self.Ing Avail Tomato`) (`self.Ing Avail Onion`) (`self.Ing Avail Beef`))
        (set `self.Ingredients Avaliable` true)
        (else
          (set `self.Ingredients Avaliable` false))))
    (:`NewEnumerator14`
      (if (and (`self.Ing Avail Buns`) (`self.Ing Avail Lettuce`) (`self.Ing Avail Tomato`) (`self.Ing Avail Onion`) (`self.Ing Avail Beef`))
        (set `self.Ingredients Avaliable` true)
        (else
          (set `self.Ingredients Avaliable` false))))
    (:`NewEnumerator15`
      (if (and (`self.Ing Avail Buns`) (`self.Ing Avail Cheese`) (`self.Ing Avail Lettuce`) (`self.Ing Avail Tomato`) (`self.Ing Avail Onion`) (`self.Ing Avail Beef`))
        (set `self.Ingredients Avaliable` true)
        (else
          (set `self.Ingredients Avaliable` false))))))

(fn `Collect Burger`
  (if (and (`self.isFull`) (`self.isDone`))
    (`/Engine/EditorBlueprintResources/StandardMacros.IncrementInt` (`self.Burger Stock`)
      (:`  `
        (`/Engine/EditorBlueprintResources/StandardMacros.IncrementInt` (`self.Total Burgers`)
          (:`  `
            (set `self.isFull` false)
            (set `self.isDone` false)))))))

(fn `Cook Logic`
  (if (`self.Ingredients Avaliable`)
    (if (`self.isFull`)
      _
      (elif (`self.isCooking`)
        _
        (elif (not (`self.isDone`))
          (set `self.isCooking` true))))))

(fn `Inc Cook Amount`
  (bind _cook_amount (`self.Cook Amount`))
  (if (`self.isCooking`)
    (if (>= _cook_amount (`self.Done Cooking`))
      (set `self.Cook Amount` 0.0)
      (set `self.isCooking` false)
      (set `self.isFull` true)
      (set `self.isDone` true)
      (else
        (set `self.Cook Amount` (+ _cook_amount (`self.Cook Increment`)))))))

(fn `Sell Burger`
  (bind _burger_stock (`self.Burger Stock`))
  (if (> _burger_stock 0)
    (`/Engine/EditorBlueprintResources/StandardMacros.DecrementInt` _burger_stock
      (:`  `
        (set `self.Cash` (+ (`self.Cash`) (`self.Burger Price`)))))))

(fn `Sell Logic`
  (for _ (range 1 (+ (`self.Customers`) 1))
    (set `self.Sell Success` (`KismetMathLibrary.RandomFloatInRange` 0.0 1.0))
    (if (>= (`self.Current Appeal`) (`self.Sell Success`))
      (`self.Sell Burger`))))

(fn `Set Public Demand`
  (set `self.Public Demand` (* (`self.Current Appeal`) 1000.0)))

(fn `Spend Ingredients`
  (if (`self.Ingredients Avaliable`)
    (`/Engine/EditorBlueprintResources/StandardMacros.DecrementInt` (`self.Buns`)
      (:`  `
        (set `self.Beef` (- (`self.Beef`) 0.5))
        (if (`self.CheeseUnlocked`)
          (`/Engine/EditorBlueprintResources/StandardMacros.DecrementInt` (`self.Cheese`)
            (:`  `
              _)))
        (if (`self.LettuceUnlocked`)
          (set `self.Lettuce` (- (`self.Lettuce`) 2)))
        (if (`self.TomatoUnlocked`)
          (set `self.Tomato` (- (`self.Tomato`) 2)))
        (if (`self.OnionUnlocked`)
          (`/Engine/EditorBlueprintResources/StandardMacros.DecrementInt` (`self.Onion`)))))))

(fn `Unlock Advertising`
  (bind _cash (`self.Cash`))
  (bind _ad_price (`self.Ad Price`))
  (switch `int` (`self.Advert Count`)
    (:`Default`
      (set `self.Ad Price` 10.0)
      (set `self.Ad Appeal Mod` 0.05))
    (:`0`
      (set `self.Ad Price` 10.0)
      (set `self.Ad Appeal Mod` 0.05))
    (:`1`
      (set `self.Ad Price` 25.0)
      (set `self.Ad Appeal Mod` 0.1))
    (:`2`
      (set `self.Ad Price` 100.0)
      (set `self.Ad Appeal Mod` 0.5))
    (:`3`
      (set `self.Ad Price` 250.0)
      (set `self.Ad Appeal Mod` 1.0))
    (:`4`
      (set `self.Ad Price` 500.0)
      (set `self.Ad Appeal Mod` 2.5))
    (:`5`
      (set `self.Ad Price` 1000.0)
      (set `self.Ad Appeal Mod` 5.0)))
  (if (>= (`KismetMathLibrary.Conv_IntToDouble` (`KismetMathLibrary.FTrunc` _cash)) _ad_price)
    (set `self.Cash` (- _cash _ad_price))
    (set `self.Base Appeal` (+ (`self.Base Appeal`) (`self.Ad Appeal Mod`)))
    (`/Engine/EditorBlueprintResources/StandardMacros.IncrementInt` (`self.Advert Count`))))

(fn `Unlock Cheese`
  (bind _cash (`self.Cash`))
  (if (>= (`KismetMathLibrary.Conv_IntToDouble` (`KismetMathLibrary.FTrunc` _cash)) 10.0)
    (set `self.Cash` (- _cash 10.0))
    (set `self.Base Appeal` (+ (`self.Base Appeal`) 0.05))
    (set `self.CheeseUnlocked` true)))

(fn `Unlock Lettuce`
  (bind _cash (`self.Cash`))
  (if (>= (`KismetMathLibrary.Conv_IntToDouble` (`KismetMathLibrary.FTrunc` _cash)) 10.0)
    (set `self.Cash` (- _cash 10.0))
    (set `self.Base Appeal` (+ (`self.Base Appeal`) 0.05))
    (set `self.LettuceUnlocked` true)))

(fn `Unlock Onion`
  (bind _cash (`self.Cash`))
  (if (>= (`KismetMathLibrary.Conv_IntToDouble` (`KismetMathLibrary.FTrunc` _cash)) 10.0)
    (set `self.Cash` (- _cash 10.0))
    (set `self.Base Appeal` (+ (`self.Base Appeal`) 0.05))
    (set `self.OnionUnlocked` true)))

(fn `Unlock Tomato`
  (bind _cash (`self.Cash`))
  (if (>= (`KismetMathLibrary.Conv_IntToDouble` (`KismetMathLibrary.FTrunc` _cash)) 10.0)
    (set `self.Cash` (- _cash 10.0))
    (set `self.Base Appeal` (+ (`self.Base Appeal`) 0.05))
    (set `self.TomatoUnlocked` true)))
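; Display sign that shows the current burger build as a 2D sprite.
; Every Tick runs AnimationLogic, which casts the game instance to BC_GameInstance and reads its BurgerStates enum.
; A switch over the base state and each combination of the C, L, T and O letters sets the matching sprite on the Burger component, polling rather than reacting to change events.
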(event `self.ReceiveTick`
  (params (DeltaSeconds :type "Float (single-precision)"))
  (`self.Animation Logic`))

(fn `Animation Logic`
  (bind _burger (`self.Burger`))
  (bind _asbc_game_instance (cast `/Game/Blueprints/BC_GameInstance` (`GameplayStatics.GetGameInstance`)))
  (switch `/Game/Blueprints/Burger_States` (`/Game/Blueprints/BC_GameInstance.Burger States` _asbc_game_instance)
    (:`NewEnumerator0`
      (`PaperSpriteComponent.SetSprite` _burger "/Game/Sprites/Burger_Sprites/BASE.BASE"))
    (:`NewEnumerator1`
      (`PaperSpriteComponent.SetSprite` _burger "/Game/Sprites/Burger_Sprites/C.C"))
    (:`NewEnumerator2`
      (`PaperSpriteComponent.SetSprite` _burger "/Game/Sprites/Burger_Sprites/L.L"))
    (:`NewEnumerator3`
      (`PaperSpriteComponent.SetSprite` _burger "/Game/Sprites/Burger_Sprites/T.T"))
    (:`NewEnumerator4`
      (`PaperSpriteComponent.SetSprite` _burger "/Game/Sprites/Burger_Sprites/O.O"))
    (:`NewEnumerator5`
      (`PaperSpriteComponent.SetSprite` _burger "/Game/Sprites/Burger_Sprites/CL.CL"))
    (:`NewEnumerator6`
      (`PaperSpriteComponent.SetSprite` _burger "/Game/Sprites/Burger_Sprites/CO.CO"))
    (:`NewEnumerator7`
      (`PaperSpriteComponent.SetSprite` _burger "/Game/Sprites/Burger_Sprites/CT.CT"))
    (:`NewEnumerator8`
      (`PaperSpriteComponent.SetSprite` _burger "/Game/Sprites/Burger_Sprites/LO.LO"))
    (:`NewEnumerator9`
      (`PaperSpriteComponent.SetSprite` _burger "/Game/Sprites/Burger_Sprites/LT.LT"))
    (:`NewEnumerator10`
      (`PaperSpriteComponent.SetSprite` _burger "/Game/Sprites/Burger_Sprites/TO.TO"))
    (:`NewEnumerator11`
      (`PaperSpriteComponent.SetSprite` _burger "/Game/Sprites/Burger_Sprites/CLO.CLO"))
    (:`NewEnumerator12`
      (`PaperSpriteComponent.SetSprite` _burger "/Game/Sprites/Burger_Sprites/CLT.CLT"))
    (:`NewEnumerator13`
      (`PaperSpriteComponent.SetSprite` _burger "/Game/Sprites/Burger_Sprites/CTO.CTO"))
    (:`NewEnumerator14`
      (`PaperSpriteComponent.SetSprite` _burger "/Game/Sprites/Burger_Sprites/LTO.LTO"))
    (:`NewEnumerator15`
      (`PaperSpriteComponent.SetSprite` _burger "/Game/Sprites/Burger_Sprites/CLTO.CLTO"))))

(fn `UserConstructionScript`)